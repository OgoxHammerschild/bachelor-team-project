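; BP_Spawner spawns the enemies of a wave at its own location.
; Its Spawn event receives wave info, loops over every EEnemy type and reads that type's count from the enemy amount map.
; The switch on type leads to spawning BP_Enemy_Meele, the only enemy class used.
; Each spawn gets a default controller and is added to BP_GameState's CurrentWave.
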(event `Spawn`
  (params (WaveInfo :type "/Game/BP_Objects/WaveSpawning/FWave Structure"))
  (bind _output_get (set `self.CurrentWaveInfo` WaveInfo))
  (bind _enumvalue (foreach `/Game/BP_Objects/WaveSpawning/EEnemy`)
    (:`LoopBody`
      (bind (_value _returnvalue) (`BlueprintMapLibrary.Map_Find` (`.Enemy_Amount_Map_8_E9B149DE4D03DBD82A109D9640B4C7B1` (break `/Game/BP_Objects/WaveSpawning/FWave` _output_get)) _enumvalue))
      (if _returnvalue
        (for _ (range 1 (+ _value 1))
          (switch `/Game/BP_Objects/WaveSpawning/EEnemy` _enumvalue
            (:`NewEnumerator0`
              (bind _returnvalue_2 (`|SpawnActorFromClass` "/Game/BP_Objects/Characters/ThirdPersonCharacter/BP_Enemy_Meele.BP_Enemy_Meele_C" (`KismetMathLibrary.Conv_VectorToTransform` (`self.K2_GetActorLocation`)) "AdjustIfPossibleButAlwaysSpawn" "OverrideRootScale"))
              (`Pawn.SpawnDefaultController` _returnvalue_2)
              (bind _asbp_game_state (cast `/Game/BP_Objects/Game/BP_GameState` (`GameplayStatics.GetGameState`)))
              (`KismetArrayLibrary.Array_Add` (`/Game/BP_Objects/Game/BP_GameState.CurrentWave` _asbp_game_state) _returnvalue_2))))))))

(fn `UserConstructionScript`)