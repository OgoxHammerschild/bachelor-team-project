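; BP_Pickup is a pickup Blueprint that animates its Pickup component with a hovering bob and a continuous spin.
; A Hover timeline starts on BeginPlay and ping-pongs between forward and reverse, adding its Z output as a local offset with separate handling for the backward pass.
; Tick applies yaw rotation scaled by delta time and RotationSpeed.
; It contains no collection logic.
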(event `self.ReceiveBeginPlay`
  (bind (_direction _z) (`Timeline|Hover` :!via `PlayFromStart` :!label _label)
    (:`Update`
      (bind _output_get (set `self.DeltaZ` _z))
      (switch `ETimelineDirection` _direction
        (:`Forward`
          _)
        (:`Backward`
          (`/Engine/EditorBlueprintResources/StandardMacros.NegateFloat` _output_get
            (:`  `
              _))))
      (`SceneComponent.K2_AddLocalOffset` (`self.Pickup`) (`KismetMathLibrary.MakeVector` 0.0 0.0 (`self.DeltaZ`)) false false))
    (:`Finished`
      (switch `ETimelineDirection` _direction
        (:`Forward`
          (goto _label :!via `Reverse`))
        (:`Backward`
          (goto _label))))))

(event `self.ReceiveTick`
  (params (DeltaSeconds :type "Float (single-precision)"))
  (`SceneComponent.K2_AddLocalRotation` (`self.Pickup`) (`KismetMathLibrary.MakeRotator` 0.0 0.0 (* DeltaSeconds (`self.RotationSpeed`))) false false))

(fn `UserConstructionScript`)